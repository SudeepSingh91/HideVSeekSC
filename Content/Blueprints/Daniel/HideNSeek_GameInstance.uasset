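; Game Instance for Hide N Seek that handles multiplayer session hosting, searching and joining through three custom events.
; Hosting creates a session with one public connection, then opens the given level as a listen server.
; Searching stores up to six LAN results in AvailableSessions, but notifies the player of a list update only when the search fails.
; Joining connects to a passed-in session, with join results and other failures printed on screen.
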(event `Instance_HostLobby`
  (params (Caller :type "PlayerController Object Reference") (Level :type Name) (useLan :type Boolean))
  ;[1 1 1] Comment
  (`CreateSessionCallbackProxy.CreateSession` Caller 1 useLan
    (:`then`
      (`GameplayStatics.OpenLevel` Level true "listen"))
    (:`OnFailure`
      (`KismetSystemLibrary.PrintString` "fail to create session" true true (struct :`R` 1.0 :`G` 0.043975 :`A` 1.0)))))

(event `Instance_JoinLobby`
  (params (Player :type "PlayerController Object Reference") (Session :type "BlueprintSessionResult Structure"))
  ;[1 1 1] Comment
  (`JoinSessionCallbackProxy.JoinSession` Player Session
    (:`OnSuccess`
      (`KismetSystemLibrary.PrintString` "Joining"))
    (:`OnFailure`
      (`KismetSystemLibrary.PrintString` "Failed to Join Session"))))

(event `Instance_UpdateAvailableSessions`
  (params (Player :type "/Game/Blueprints/Daniel/Lobby/LobbyPlayerController Object Reference"))
  ;[1 1 1] Comment
  (bind _results (`FindSessionsCallbackProxy.FindSessions` Player 6 true)
    (:`then`
      (set `self.AvailableSessions` _results))
    (:`OnFailure`
      (`KismetSystemLibrary.PrintString` "Session search failed" true true (struct :`R` 1.0 :`G` 0.028582 :`A` 1.0))
      (`/Game/Blueprints/Daniel/Lobby/LobbyPlayerController.NotifySessionListUpdated` Player)
      (`KismetSystemLibrary.PrintString` "SessionListUpdated"))))