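; Game instance for a hide-and-seek game that hosts, finds and joins sessions and opens tutorial levels.
; Hosting creates a two-connection session, opens the map as a listen server, and saves room name, password, mode and map to a SaveGame slot named after the player controller.
; Session search is LAN-only and reloads local save slots to print room names, using each result's player count as the controller index.
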(event `Instance_HostLobby`
  (params (GameMap :type String) (useLan :type Boolean) (RoomName :type Text) (RoomPassword :type Text) (GameMode :type String) (PlayerController :type "PlayerController Object Reference"))
  ;[1 1 1] Comment
  (`CreateSessionCallbackProxy.CreateSession` PlayerController 2 useLan
    (:`OnSuccess`
      (`GameplayStatics.OpenLevel` (`KismetStringLibrary.Conv_StringToName` GameMap) true "listen")
      (`GameplayStatics.CreateSaveGameObject` "/Game/UI/MainMenu/SaveSessionInfo.SaveSessionInfo_C")
      (set `self.SaveInfo` null)
      (bind _assave_session_info (cast `/Game/UI/MainMenu/SaveSessionInfo` null))
      (set `/Game/UI/MainMenu/SaveSessionInfo.RoomName` RoomName _assave_session_info)
      (set `/Game/UI/MainMenu/SaveSessionInfo.RoomPassword` RoomPassword _assave_session_info)
      (bind _output_get (set `/Game/UI/MainMenu/SaveSessionInfo.GameMode` GameMode _assave_session_info))
      (set `/Game/UI/MainMenu/SaveSessionInfo.GameMap` GameMap _assave_session_info)
      (`GameplayStatics.SaveGameToSlot` null (`KismetSystemLibrary.GetDisplayName` PlayerController)))
    (:`OnFailure`
      (`KismetSystemLibrary.PrintString` "fail to create session" true true (struct :`R` 1.0 :`G` 0.043975 :`A` 1.0) 10.0))))

(event `Instance_JoinLobby`
  (params (PlayerController :type "PlayerController Object Reference") (Session :type "BlueprintSessionResult Structure"))
  ;[1 1 1] Comment
  (`JoinSessionCallbackProxy.JoinSession` PlayerController Session
    (:`OnSuccess`
      (`KismetSystemLibrary.PrintString` "Joining"))
    (:`OnFailure`
      (`KismetSystemLibrary.PrintString` "Failed to Join Session"))))

(event `Instance_UpdateAvailableSessions`
  (params (PlayerController :type "PlayerController Object Reference"))
  ;[1 1 1] Comment
  (bind _results (`FindSessionsCallbackProxy.FindSessions` PlayerController 6 true)
    (:`OnSuccess`
      (set `self.Serverlist` _)
      (for _array_element _results
        (`GameplayStatics.LoadGameFromSlot` (`KismetSystemLibrary.GetDisplayName` (`GameplayStatics.GetPlayerController` (`FindSessionsCallbackProxy.GetCurrentPlayers` _array_element))))
        (set `self.SaveInfo` null)
        (bind _assave_session_info (cast `/Game/UI/MainMenu/SaveSessionInfo` null))
        (`KismetSystemLibrary.PrintString` (`KismetTextLibrary.Conv_TextToString` (`/Game/UI/MainMenu/SaveSessionInfo.RoomName` _assave_session_info)) true true (struct :`G` 0.66 :`B` 1.0 :`A` 1.0) 10.0)))
    (:`OnFailure`
      (`KismetSystemLibrary.PrintString` "Session search failed" true true (struct :`R` 1.0 :`G` 0.028582 :`A` 1.0)))))

(event `OpenTutorial`
  (params (Level :type Name))
  ;[1 1 1] Comment
  (`GameplayStatics.OpenLevel` Level true "listen"))