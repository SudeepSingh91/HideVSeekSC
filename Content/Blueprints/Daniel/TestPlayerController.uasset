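; Test player controller for the Hide N Seek game that forwards lobby hosting, joining and session refresh requests to HideNSeek_GameInstance.
; Hosting runs only with authority and sets Game and UI input; joining passes the controller and ignores its Session input.
; After a short delay, BeginPlay calls a HUD creation event on authority, but that event is empty and the lobby menu visibility logic is disconnected.
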(event `self.ReceiveBeginPlay`
  (`KismetSystemLibrary.Delay` 0.2)
  (`/Engine/EditorBlueprintResources/ActorMacros.Switch Has Authority`
    (:`Authority`
      (`self.Player_Client_CreateHUD`))))

(event `Player_Client_CreateHUD`)

(event `Player_HostMap`
  (`self.HostLobby` self "None"))

(event `Player_JoinServer`
  (`self.JoinLobby` :`self` self))

(fn `HostLobby`
  (params (LevelName :type Name))
  (`/Engine/EditorBlueprintResources/ActorMacros.Switch Has Authority`
    (:`Authority`
      (bind _ashide_nseek_game_instance (cast `/Game/Blueprints/Daniel/HideNSeek_GameInstance` (`GameplayStatics.GetGameInstance`)))
      (`/Game/Blueprints/Daniel/HideNSeek_GameInstance.Instance_HostLobby` _ashide_nseek_game_instance null LevelName false)
      (`WidgetBlueprintLibrary.SetInputMode_GameAndUIEx` self))))

(fn `JoinLobby`
  (params (Session :type "BlueprintSessionResult Structure"))
  (bind _ashide_nseek_game_instance (cast `/Game/Blueprints/Daniel/HideNSeek_GameInstance` (`GameplayStatics.GetGameInstance`)))
  (`/Game/Blueprints/Daniel/HideNSeek_GameInstance.Instance_JoinLobby` :`self` _ashide_nseek_game_instance :`Player` self))

(fn `SwitchLobbyHUDVisibilty`)

(fn `UpdateAvilableSessions`
  (bind _ashide_nseek_game_instance (cast `/Game/Blueprints/Daniel/HideNSeek_GameInstance` (`GameplayStatics.GetGameInstance`)))
  (`/Game/Blueprints/Daniel/HideNSeek_GameInstance.Instance_UpdateAvailableSessions` _ashide_nseek_game_instance null))

(fn `UserConstructionScript`)