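; Test player character for trying out movement, interaction and HUD features such as health, ability cooldowns, pause and elimination widgets.
; Input drives movement, look, component activation through a server-named event, and debug keys.
; A damage-test input briefly reveals the 3D health widget, which Tick yaws toward player zero.
; Ability inputs run timelines that lerp cooldown values behind ready flags, while separate countdown events and getter functions supply display data.
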(event `InputAction|Interact`
  (params (Key :type "Key Structure" :default "AnyKey"))
  ;[1 1 1] RayCast Event
  (:`Pressed`
    (`self.SRV_onUsed`)))

(event `Toogle`
  (`KismetSystemLibrary.PrintString` "toogling")
  (`SceneComponent.SetVisibility` (`self.3dHealthWidget`) true true)
  (`KismetSystemLibrary.Delay` 1.0)
  (`SceneComponent.SetVisibility` (`self.3dHealthWidget`) false true))

(event `Toogle_server`
  (`KismetSystemLibrary.PrintString` "toogling")
  (`SceneComponent.SetVisibility` (`self.3dHealthWidget`) true true)
  (`KismetSystemLibrary.Delay` 1.0)
  (`SceneComponent.SetVisibility` (`self.3dHealthWidget`) false true))

(event `InputAxis|MoveForward`
  (params (AxisValue :type "Float (single-precision)"))
  ;[1 1 1] Input
  (`self.AddMovementInput` (`KismetMathLibrary.GetForwardVector` (`self.GetControlRotation`)) AxisValue))

(event `SRV_onUsed`
  ;[1 1 1] RayCast Event
  (`/Game/Blueprints/Arpit/DoornSwitch/ActivateStuffComponent.TryActivate` (`self.ActivateStuffComponent`)))

(event `self.ReceiveBeginPlay`
  (`SceneComponent.SetVisibility` (`self.3dHealthWidget`) false false))

(event `InputAxis|MoveRight`
  (params (AxisValue :type "Float (single-precision)"))
  ;[1 1 1] Input
  (`self.AddMovementInput` (`KismetMathLibrary.GetRightVector` (`self.GetControlRotation`)) AxisValue))

(event `InputAction|TestDamage`
  (params (Key :type "Key Structure" :default "AnyKey"))
  (:`Pressed`
    (`self.Toogle`)
    (`self.Toogle_server`)))

(event `InputAxis|LookUp`
  (params (AxisValue :type "Float (single-precision)"))
  ;[1 1 1] Input
  (`self.AddControllerPitchInput` AxisValue))

(event `InputAxis|LookHorizontal`
  (params (AxisValue :type "Float (single-precision)"))
  ;[1 1 1] Input
  (`self.AddControllerYawInput` AxisValue))

(event `self.ReceiveTick`
  (params (DeltaSeconds :type "Float (single-precision)"))
  (bind _3dhealthwidget (`self.3dHealthWidget`))
  ;[1 1 1] Set the location of health bar on screen
  (`SceneComponent.K2_SetWorldRotation` _3dhealthwidget (`KismetMathLibrary.MakeRotator` 0.0 0.0 (.yaw (`KismetMathLibrary.FindLookAtRotation` (`SceneComponent.K2_GetComponentLocation` _3dhealthwidget) (`self.K2_GetActorLocation` (`GameplayStatics.GetPlayerCharacter` 0))))) false false))

(event `Key|N`
  (params (Key :type "Key Structure" :default "AnyKey"))
  (:`Pressed`
    (bind _returnvalue (`|CreateWidget` "/Game/Blueprints/Arpit/Elimination_widget.Elimination_widget_C" (`GameplayStatics.GetPlayerController` 0)))
    (`UserWidget.AddToViewport` _returnvalue 0)))

(event `Key|M`
  (params (Key :type "Key Structure" :default "AnyKey"))
  (bind _objectivenumbers (`self.ObjectiveNumbers`))
  (:`Pressed`
    (if (< _objectivenumbers 3)
      (set `self.ObjectiveNumbers` (+ _objectivenumbers 1)))))

(event `InputAction|Pause`
  (params (Key :type "Key Structure" :default "AnyKey"))
  (bind _returnvalue (`GameplayStatics.GetPlayerController` 0))
  ;[1 1 1] Disable player input when paused
  (:`Pressed`
    (`self.DisableInput` (`GameplayStatics.GetPlayerCharacter` 0) _returnvalue)
    (bind _returnvalue_2 (`|CreateWidget` "/Game/Blueprints/Arpit/Pause_Menu.Pause_Menu_C" _returnvalue))
    (`UserWidget.AddToViewport` _returnvalue_2 0)
    (`WidgetBlueprintLibrary.SetInputMode_GameAndUIEx` _returnvalue _returnvalue_2 true)))

(event `InputAction|Ability1`
  (params (Key :type "Key Structure" :default "AnyKey"))
  ;[1 1 1] Change the UI after pressing the ability1/ability2 buttons
  (:`Pressed`
    (if (`self.CooldownDelay`)
      (set `self.CooldownDelay` false)
      (set `self.TestCoolDown` 100.0)
      (bind (_direction _getback) (`Timeline|Timeline_Ability1SetBack` :!via `PlayFromStart`)
        (:`Update`
          (set `self.TestCoolDown` (`KismetMathLibrary.Lerp` 100.0 0.0001 _getback)))
        (:`Finished`
          (set `self.CooldownDelay` true))))))

(event `InputAction|Ability2`
  (params (Key :type "Key Structure" :default "AnyKey"))
  ;[1 1 1] Change the UI after pressing the ability1/ability2 buttons
  (:`Pressed`
    (if (`self.SecondCoolDownDelay`)
      (set `self.SecondCoolDownDelay` false)
      (set `self.TestCoolDown2` 100.0)
      (bind (_direction _getback) (`Timeline|Timeline_Ability2SetBack` :!via `PlayFromStart`)
        (:`Update`
          (set `self.TestCoolDown2` (`KismetMathLibrary.Lerp` 100.0 0.0001 _getback)))
        (:`Finished`
          (set `self.SecondCoolDownDelay` true))))))

(event `Ability1Coooldown`
  (`KismetSystemLibrary.Delay` 1.0 :!label _label)
  (bind _output_get (set `self.CooldownTimer` (- (`self.CooldownTimer`) 1)))
  (if (< _output_get 0)
    (set `self.CooldownTimer` 3)
    (else
      (goto _label))))

(event `Ability2Coooldown`
  (`KismetSystemLibrary.Delay` 1.0 :!label _label_2)
  (bind _output_get (set `self.SecondCooldownTimer` (- (`self.SecondCooldownTimer`) 1)))
  (if (< _output_get 0)
    (set `self.SecondCooldownTimer` 3)
    (else
      (goto _label_2))))

(fn `AbilityTextDisplay`
  (returns (CurrentStatus :type String))
  ;[1 1 1] Get the text for ability 1
  (if (`self.CooldownDelay`)
    (return (`KismetStringLibrary.Conv_IntToString` (`self.CooldownTimer`)))
    (else
      (return (`self.Ability1`)))))

(fn `HealthState`
  (returns (CurrentHealth :type "Float (double-precision)") (MaxHealth :type "Float (double-precision)"))
  ;[1 1 1] Get the health
  (return (`self.CurrentHealth`) (`self.MaxHealth`)))

(fn `SecondAbilityTextDisplay`
  (returns (SecondCurrentStatus :type String))
  ;[1 1 1] Get the text for ability 2
  (if (`self.SecondCoolDownDelay`)
    (return (`KismetStringLibrary.Conv_IntToString` (`self.SecondCooldownTimer`)))
    (else
      (return (`self.Ability2`)))))

(fn `UserConstructionScript`)