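; WaterBalloon is an actor that bursts on impact to damage nearby Hiders.
; When its static mesh registers a hit, the authority side runs a sphere overlap at the impact point and calls ReceiveDamage on each Hider found.
; It then plays a grenade reveal sound, spawns a Shockwave actor at that point and destroys itself through the Explode event.
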(event `self.StaticMeshComponent.OnComponentHit`
  (params (HitComponent :type "PrimitiveComponent Object Reference") (OtherActor :type "Actor Object Reference") (OtherComp :type "PrimitiveComponent Object Reference") (NormalImpulse :type "Vector Structure") (Hit :type "HitResult Structure (by ref)"))
  (bind (_bblockinghit _binitialoverlap _time _location) (`GameplayStatics.BreakHitResult` Hit))
  ;[1 1 1] Hider Detection
  (`/Engine/EditorBlueprintResources/ActorMacros.Switch Has Authority`
    (:`Authority`
      (bind _outactors (`KismetSystemLibrary.SphereOverlapActors_NEW` _location 150.0 (`|MakeArray` "ObjectTypeQuery2" "ObjectTypeQuery3" :!type "EObjectTypeQuery Enum")))
      (for _array_element _outactors
        (bind _ashider (cast `/Game/HiderBP/Blueprints/Hider` _array_element))
        (`/Game/HiderBP/Blueprints/Hider.ReceiveDamage` _ashider 110))
      (`GameplayStatics.PlaySoundAtLocation` "/Game/Sounds/16_bit_Grenade__Reveal_.16_bit_Grenade__Reveal_" _location)
      (`|SpawnActorFromClass` "/Game/Blueprints/Sudeep/shockwave.shockwave_C" (`KismetMathLibrary.MakeTransform` _location) "AlwaysSpawn" "OverrideRootScale")
      (`self.Explode`))))

(event `self.ReceiveActorBeginOverlap`
  (params (OtherActor :type "Actor Object Reference")))

(event `Explode`
  ;[1 1 1] Explode
  (`self.K2_DestroyActor`))

(fn `UserConstructionScript`)