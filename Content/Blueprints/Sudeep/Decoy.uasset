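; Decoy actor that copies the mesh of its Hider's current object on BeginPlay.
; If the Hider is moving at that moment, it picks a random, normalized horizontal direction with positive local X.
; Tick then slides it by a fixed, unswept local offset per frame, not scaled by delta time.
; A mesh overlap with anything not display-named "Floor" stops the movement.
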(event `self.ReceiveBeginPlay`
  (bind _hider (`self.Hider`))
  ;[1 1 1] Generate Mesh for Decoy
  (`StaticMeshComponent.SetStaticMesh` (`self.StaticMesh`) (`/Game/Blueprints/Sudeep/HiderAbilities_ray11.Current_Object` (`/Game/HiderBP/Blueprints/Hider.HiderAbilities` _hider)))
  (if (not (== (`KismetMathLibrary.VSize` (`self.GetVelocity` _hider)) 0.0))
    (set `self.Can_Move` true)
    (set `self.DirVec` (* (`KismetMathLibrary.Normal` (`KismetMathLibrary.MakeVector` 1.0 (`KismetMathLibrary.RandomFloatInRange` -3.0 3.0))) 18))))

(event `self.StaticMesh.OnComponentBeginOverlap`
  (params (OverlappedComponent :type "PrimitiveComponent Object Reference") (OtherActor :type "Actor Object Reference") (OtherComp :type "PrimitiveComponent Object Reference") (OtherBodyIndex :type Integer) (bFromSweep :type Boolean) (SweepResult :type "HitResult Structure (by ref)"))
  ;[1 1 1] Stop Moving On Collision
  (if (not (`KismetStringLibrary.EqualEqual_StrStr` (`KismetSystemLibrary.GetDisplayName` OtherActor) "Floor"))
    (set `self.Can_Move` false)))

(event `self.ReceiveTick`
  (params (DeltaSeconds :type "Float (single-precision)"))
  ;[1 1 1] Update Position
  (if (`self.Can_Move`)
    (`self.K2_AddActorLocalOffset` (`self.DirVec`))))

(fn `UserConstructionScript`)