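; Ability component for the Seeker character that fires paint grenades, temporary invisibility via material swap, trap decoys and ammo throwables.
; AbilityID and AmmoID select the action, with projectiles spawned at "Launch"-tagged components facing "Aim"-tagged meshes.
; For decoys, CheckForCooldown stores a random nearby ReplaceableMeshActor's mesh as TrapMesh before firing.
; Only TriggerAbility1 is implemented, firing paint grenades behind a delay gate; other triggers are empty and several chains are unwired.
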(event `CheckForCooldown`
  (bind _returnvalue (`self.GetOwner`))
  ;[1 1 1] Check Cooldown
  (if (== (`self.Ability_Available`) true)
    (if (== (`self.AbilityID`) 2)
      (bind (_outactors _returnvalue_2) (`KismetSystemLibrary.SphereOverlapActors_NEW` (+ (+ (`Actor.K2_GetActorLocation` _returnvalue) (0.0 0.0 -70.0)) (* (`KismetMathLibrary.GetForwardVector` (`Actor.K2_GetActorRotation` _returnvalue)) 150)) 500.0 (`|MakeArray` "ObjectTypeQuery1" "ObjectTypeQuery2" :!type "EObjectTypeQuery Enum")))
      (if _returnvalue_2
        (bind _output_get (set `self.RandSelection` (`KismetMathLibrary.RandomIntegerInRange` 0 (- (`KismetArrayLibrary.Array_Length` _outactors) 1))))
        (for (_array_element _array_index) _outactors
          (if (== _output_get _array_index)
            (bind _asreplaceable_mesh_actor (cast `/Game/Blueprints/Daniel/RandomObjectsRoom/ReplaceableMeshActor` _array_element))
            (for _array_element_2 (`Actor.K2_GetComponentsByClass` _asreplaceable_mesh_actor "/Script/Engine.StaticMeshComponent")
              (set `self.TrapMesh` (`StaticMeshComponent.StaticMesh` _array_element_2))
              (`self.ApplyCooldown` :!label _label)
              (`self.Fire_Ability`)))))
      (else
        (goto _label)))))

(event `Reset0`
  ;[1 1 1] Cooldown Over
  (set `self.Ability_Available` true))

(event `ApplyCooldown`
  ;[1 1 1] Apply Cooldown
  (set `self.Ability_Available` false)
  (`KismetSystemLibrary.K2_SetTimerDelegate` (`|CreateDelegate` :!event `Reset0`) 3.0))

(event `TriggerAbility1`
  ;[1 1 1] Trigger Abilities
  (if (`self.Temp1`)
    (set `self.Temp1` false)
    (set `self.AbilityID` 0)
    (`self.Fire_Ability`)
    (`KismetSystemLibrary.Delay` 15.0)
    (set `self.Temp1` true)))

(event `TriggerAbility2`
  ;[1 1 1] Trigger Abilities
)

(event `TriggerUltimate`
  ;[1 1 1] Trigger Abilities
)

(event `SetTransparency`
  (params (StaticMesh :type "StaticMeshComponent Object Reference"))
  ;[1 1 1] Set Transparency
  (`PrimitiveComponent.SetMaterial` StaticMesh 0 "/Game/SeekerBP/Blueprints/SeekerBlinn1SG1.SeekerBlinn1SG1")
  (`KismetSystemLibrary.Delay` 5.0)
  (`self.ResetTransparency` StaticMesh))

(event `CheckForAmmo`
  (bind _ammo_available (`self.Ammo_Available`))
  ;[1 1 1] Check For Ammo
  (if (> _ammo_available 0)
    (set `self.Ammo_Available` (- _ammo_available 1))
    (`self.FireAmmo`)))

(event `ResetTransparency`
  (params (`Static Mesh` :type "StaticMeshComponent Object Reference"))
  ;[1 1 1] Set Transparency
  (`PrimitiveComponent.SetMaterial` `Static Mesh` 0 "/Game/SeekerBP/Blueprints/blinn1SG1.blinn1SG1"))

(fn `Fire_Ability`
  (bind _returnvalue (`self.GetOwner`))
  (bind _returnvalue_2 (`self.GetOwner`))
  ;[1 1 1] Firing of Abilities and Cooldown
  (for _array_element (`Actor.GetComponentsByTag` _returnvalue_2 "/Script/Engine.StaticMeshComponent" "Pivot")
    _)
  (bind _asstatic_mesh_component (cast `StaticMeshComponent` _array_element))
  (for _array_element_2 (`Actor.GetComponentsByTag` _returnvalue_2 "/Script/Engine.ChildActorComponent" "Launch")
    _)
  (switch `int` (`self.AbilityID`)
    (:`0`
      (`self.PaintGrenade`))
    (:`1`
      (`self.Invisible`))
    (:`2`
      (`|SpawnActorFromClass` "/Game/Blueprints/Sudeep/Trap_Decoy.Trap_Decoy_C" (`KismetMathLibrary.MakeTransform` (+ (- (`Actor.K2_GetActorLocation` _returnvalue) (0.0 0.0 110.0)) (* (`KismetMathLibrary.GetForwardVector` (`Actor.K2_GetActorRotation` _returnvalue)) 150)) (struct) (1.0 1.0 1.0)) "AlwaysSpawn" "OverrideRootScale"))))

(fn `FireAmmo`
  ;[1 1 1] Fire Ammo
  (switch `int` (`self.AmmoID`)
    (:`0`
      (`self.TrapGrenade`))
    (:`1`
      (`self.PaintGrenade`))))

(fn `Grenade`
  (bind _returnvalue (`self.GetOwner`))
  ;[1 1 1] Grenade
  (for _array_element (`Actor.GetComponentsByTag` _returnvalue "/Script/Engine.ChildActorComponent" "Launch")
    _)
  (for _array_element_2 (`Actor.GetComponentsByTag` _returnvalue "/Script/Engine.StaticMeshComponent" "Aim")
    _)
  (bind _asstatic_mesh_component (cast `StaticMeshComponent` _array_element_2))
  (bind _returnvalue_2 (`SceneComponent.K2_GetComponentLocation` _array_element))
  (`|SpawnActorFromClass` "/Game/Blueprints/Sudeep/Grenade.Grenade_C" (`KismetMathLibrary.MakeTransform` _returnvalue_2 (`KismetMathLibrary.FindLookAtRotation` _returnvalue_2 (`SceneComponent.K2_GetComponentLocation` _asstatic_mesh_component)) (0.5 0.5 0.5)) "Undefined" "OverrideRootScale"))

(fn `Invisible`
  (bind _asseeker (cast `/Game/SeekerBP/Blueprints/Seeker` (`self.GetOwner`)))
  (for _array_element (`Actor.GetComponentsByTag` _asseeker "/Script/Engine.StaticMeshComponent" "Model")
    _)
  (`self.SetTransparency` _array_element))

(fn `PaintGrenade`
  (bind _returnvalue (`self.GetOwner`))
  ;[1 1 1] Paint Grenade
  (for _array_element (`Actor.GetComponentsByTag` _returnvalue "/Script/Engine.ChildActorComponent" "Launch")
    _)
  (for _array_element_2 (`Actor.GetComponentsByTag` _returnvalue "/Script/Engine.StaticMeshComponent" "Aim")
    _)
  (bind _asstatic_mesh_component (cast `StaticMeshComponent` _array_element_2))
  (bind _returnvalue_2 (`SceneComponent.K2_GetComponentLocation` _array_element))
  (`|SpawnActorFromClass` "/Game/Blueprints/Sudeep/Paint_Grenade.Paint_Grenade_C" (`KismetMathLibrary.MakeTransform` _returnvalue_2 (`KismetMathLibrary.FindLookAtRotation` _returnvalue_2 (`SceneComponent.K2_GetComponentLocation` _asstatic_mesh_component)) (0.5 0.5 0.5)) "AlwaysSpawn" "OverrideRootScale"))

(fn `TrapGrenade`
  (bind _returnvalue (`self.GetOwner`))
  ;[1 1 1] Trap Grenade
  (for _array_element (`Actor.GetComponentsByTag` _returnvalue "/Script/Engine.StaticMeshComponent" "Aim")
    _)
  (bind _asstatic_mesh_component (cast `StaticMeshComponent` _array_element))
  (for _array_element_2 (`Actor.GetComponentsByTag` _returnvalue "/Script/Engine.ChildActorComponent" "Launch")
    _)
  (bind _returnvalue_2 (`SceneComponent.K2_GetComponentLocation` _array_element_2))
  (`|SpawnActorFromClass` "/Game/Blueprints/Sudeep/Trap_Grenade.Trap_Grenade_C" (`KismetMathLibrary.MakeTransform` _returnvalue_2 (`KismetMathLibrary.FindLookAtRotation` _returnvalue_2 (`SceneComponent.K2_GetComponentLocation` _asstatic_mesh_component)) (0.5 0.5 0.5)) "Undefined" "OverrideRootScale"))

(fn `WaterBalloon`
  (bind _returnvalue (`self.GetOwner`))
  ;[1 1 1] Water Balloon
  (for _array_element (`Actor.GetComponentsByTag` _returnvalue "/Script/Engine.ChildActorComponent" "Launch")
    _)
  (for _array_element_2 (`Actor.GetComponentsByTag` _returnvalue "/Script/Engine.StaticMeshComponent" "Aim")
    _)
  (bind _asstatic_mesh_component (cast `StaticMeshComponent` _array_element_2))
  (bind _returnvalue_2 (`SceneComponent.K2_GetComponentLocation` _array_element))
  (`|SpawnActorFromClass` "/Game/Blueprints/Sudeep/WaterBalloon.WaterBalloon_C" (`KismetMathLibrary.MakeTransform` _returnvalue_2 (`KismetMathLibrary.FindLookAtRotation` _returnvalue_2 (`SceneComponent.K2_GetComponentLocation` _asstatic_mesh_component)) (0.5 0.5 0.5)) "Undefined" "OverrideRootScale"))