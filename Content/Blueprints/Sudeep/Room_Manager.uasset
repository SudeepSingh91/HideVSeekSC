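; Room manager Blueprint that randomizes a set of room objects at the start of play.
; On BeginPlay, the authority gives each room a random TargetMesh from MeshArray, removing each pick so no entry is reused.
; A position shuffle caches room locations and redistributes them without repeats through ReplicatePos, but its SetupArray and SetRoomPos calls are disconnected and never run.
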(event `SetupArray`
  (for _array_element (`self.RoomObj`)
    (`KismetArrayLibrary.Array_Add` (`self.RoomVec`) (`self.K2_GetActorLocation` _array_element))))

(event `SetRoomPos`
  (bind _roomvec (`self.RoomVec`))
  (for _index (range (`KismetArrayLibrary.Array_Length` (`self.RoomObj`)))
    (bind _output_get (set `self.IterPos` (`KismetArrayLibrary.Array_Get` _roomvec (`KismetMathLibrary.RandomIntegerInRange` 0 (- (`KismetArrayLibrary.Array_Length` _roomvec) 1)))))
    (`KismetArrayLibrary.Array_RemoveItem` (`self.RoomVec`) _output_get)
    (`self.ReplicatePos` (`KismetArrayLibrary.Array_Get` (`self.RoomObj`) _index) _output_get)))

(event `ReplicatePos`
  (params (Obj :type "/Game/Blueprints/Daniel/RandomObjectsRoom/ReplaceableMeshActor Object Reference") (Pos :type "Vector Structure"))
  (`self.K2_SetActorLocation` Obj Pos false false))

(event `self.ReceiveBeginPlay`
  (bind _returnvalue (`KismetArrayLibrary.Array_Length` (`self.MeshArray`)))
  (`/Engine/EditorBlueprintResources/ActorMacros.Switch Has Authority`
    (:`Authority`
      (if (> _returnvalue 0)
        (for _array_element (`self.RoomObj`)
          (bind _output_get (set `self.IterAct` (`KismetMathLibrary.RandomIntegerInRange` 0 (- _returnvalue 1))))
          (set `/Game/Blueprints/Daniel/RandomObjectsRoom/ReplaceableMeshActor.TargetMesh` (`KismetArrayLibrary.Array_Get` (`self.MeshArray`) _output_get) _array_element)
          (`KismetArrayLibrary.Array_Remove` (`self.MeshArray`) (`self.IterAct`)))))))

(fn `UserConstructionScript`)