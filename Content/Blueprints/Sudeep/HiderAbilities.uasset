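; Hider ability component for a prop-hunt style game, handling mesh disguises and abilities.
; The owner gets a random starting mesh and morphs into traced props from its allowed list or into decoy meshes, with ForceSwitch rerolling it.
; AbilityID selects smoke screen, temporary invisibility or an ultimate copying the disguise onto nearby replaceable props.
; AmmoID selects smoke or silence trap, with cooldown and ammo checks partly disconnected.
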(event Custom|CheckForAmmo
  ;[1 1 1] Check For Ammo
  (if (== (Variables|Default|GetAmmoID) 1)
    (if (== (.Z (Math|Vector|BreakVector (Transformation|GetVelocity (Components|GetOwner)))) 0.0)
      (if (> (Variables|Default|GetAmmo_Available) 0) :!label _label
        (Variables|Default|SetAmmo_Available (- (Variables|Default|GetAmmo_Available) 1))
        (CallFunction|FireAmmo)))
    (else
      (goto _label))))

(event Custom|MakeVisible
  (params (Static%20Mesh :type Static%20Mesh%20Component%20Object%20Reference))
  ;[1 1 1] Set Visible
  (Rendering|SetVisibility Static%20Mesh true false))

(event Custom|TriggerAbility1
  ;[1 1 1] Trigger Abilities
  (if (Variables|Default|GetTemp1)
    (Variables|Default|SetTemp1 false)
    (Variables|Default|SetAbilityID 0)
    (CallFunction|FireAbility)
    (Utilities|FlowControl|Delay 15.0)
    (Variables|Default|SetTemp1 true)))

(event Custom|ChangeMesh
  ;[1 1 1] Change the mesh
  (CallFunction|SwitchMesh))

(event Custom|TriggerAbility2
  ;[1 1 1] Trigger Abilities
)

(event Custom|TriggerUltimate
  ;[1 1 1] Trigger Abilities
  (Variables|Default|SetAbilityID 2))

(event Custom|AssignInitialMesh
  (bind _random_objects (Variables|Default|GetRandom_Objects))
  ;[1 1 1] Call Initial Mesh
  (CallFunction|MeshSwap (Utilities|Array|Get(acopy) _random_objects (Math|Random|RandomIntegerinRange 0 (- (Utilities|Array|Length _random_objects) 1)))))

(event Custom|CheckForCooldown
  (bind _returnvalue (Components|GetOwner))
  (bind _returnvalue_2 (Transformation|GetActorLocation _returnvalue))
  (bind (_x _y) (Math|Vector|BreakVector _returnvalue_2))
  ;[1 1 1] Check Cooldown
  (if (Math|Boolean|Equal(Boolean) (Variables|Default|GetAbility_Available) true)
    (if (== (Variables|Default|GetAbilityID) 0)
      (for _array_element (Actor|GetComponentsByClass _returnvalue "/Script/Engine.CameraComponent")
        (bind _returnvalue_3 (Class|KismetSystemLibrary|BoxOverlapActorsNEW (+ (+ _returnvalue_2 "0.000000,0.000000,-70.000000") (* (Math|Vector|Normalize (- (Math|Vector|MakeVector _x _y 0.0) (Math|Vector|MakeVector (.X (Math|Vector|BreakVector (Transformation|GetWorldLocation _array_element))) (.Y (Math|Vector|BreakVector (Transformation|GetWorldLocation _array_element))) 0.0))) 150)) "40.000000,40.000000,20.000000" (Utilities|Array|MakeArray "ObjectTypeQuery1" "ObjectTypeQuery2")))
        (if (not _returnvalue_3)
          (if (== (.Z (Math|Vector|BreakVector (Transformation|GetVelocity (Components|GetOwner)))) 0.0)
            (CallFunction|ApplyCooldown)
            (CallFunction|FireAbility))))
      (else
        (CallFunction|ApplyCooldown)
        (CallFunction|FireAbility)))))

(event Custom|ApplyCooldown
  ;[1 1 1] Apply Cooldown
  (Variables|Default|SetAbility_Available false)
  (Utilities|Time|SetTimerbyEvent (EventDispatchers|CreateEvent :!event Custom|Reset0) 15.0))

(event Custom|Reset0
  ;[1 1 1] Cooldown Over
  (Variables|Default|SetAbility_Available true))

(event Custom|MakeInvisible
  (params (Static%20Mesh :type Static%20Mesh%20Component%20Object%20Reference))
  ;[1 1 1] Set Visible
  (Rendering|SetVisibility Static%20Mesh false false)
  (Utilities|FlowControl|Delay 3.0)
  (CallFunction|MakeVisible Static%20Mesh))

(event Custom|MeshSwap
  (params (Mesh :type Static%20Mesh%20Object%20Reference))
  ;[1 1 1] Swap Mesh
  (bind _output_get (Variables|Default|SetCurrent_Object Mesh))
  (Components|StaticMesh|SetStaticMesh (Variables|Default|GetOwnersMesh) _output_get))

(event Custom|UltimateSwap
  (params (Mesh :type Static%20Mesh%20Component%20Object%20Reference))
  ;[1 1 1] Ultimate Swap
  (Components|StaticMesh|SetStaticMesh Mesh (Variables|Default|GetCurrent_Object)))

(fn ForceSwitch
  (bind _random_objects (Variables|Default|GetRandom_Objects))
  ;[1 1 1] Force Switch on Grenade Impact
  (while (== (stale _output_get) (Variables|/Script/Engine.StaticMeshComponent|GetStaticMesh (Variables|Default|GetOwnersMesh)))
    (bind _output_get (Variables|Default|SetCurrent_Object (Utilities|Array|Get(acopy) _random_objects (Math|Random|RandomIntegerinRange 0 (- (Utilities|Array|Length _random_objects) 1))))))
  (CallFunction|MeshSwap (Variables|Default|GetCurrent_Object)))

(fn FireAbility
  ;[1 1 1] Firing of Abilities and Cooldown
  (switch int (Variables|Default|GetAbilityID)
    (:0
      (CallFunction|SmokeScreen))
    (:1
      (CallFunction|Invisible))
    (:2
      (bind _outactors (Class|KismetSystemLibrary|SphereOverlapActorsNEW (Transformation|GetActorLocation (Components|GetOwner)) 5e+02 (Utilities|Array|MakeArray "ObjectTypeQuery2" "ObjectTypeQuery1")))
      (for _array_element _outactors
        (bind _asreplaceable_mesh_actor (Utilities|Casting|CastToReplaceableMeshActor _array_element))
        (for _array_element_2 (Actor|GetComponentsByClass _asreplaceable_mesh_actor "/Script/Engine.StaticMeshComponent")
          (CallFunction|UltimateSwap _array_element_2))))))

(fn SwitchMesh
  ;[1 1 1] Switching Mesh
  (for _array_element (Actor|GetComponentsByClass (Components|GetOwner) "/Script/Engine.CameraComponent")
    (bind _outactors (Actor|GetAllActorsOfClass "/Game/Blueprints/Sudeep/Target.Target_C"))
    (bind _outhit (Collision|LineTraceForObjects (Transformation|GetActorLocation (Components|GetOwner)) (+ (Transformation|GetWorldLocation _array_element) (* (Math|Vector|GetForwardVector (.Rotation (Math|Transform|BreakTransform (Transformation|GetWorldTransform _array_element)))) 1000)) (Utilities|Array|MakeArray "ObjectTypeQuery1" "ObjectTypeQuery2") false _outactors "None"))
    (bind _asstatic_mesh_actor (Utilities|Casting|CastToStaticMeshActor (.HitActor (Collision|BreakHitResult _outhit)))
      (:then
        (LocalVariables|SetstaticMesh (Variables|/Script/Engine.StaticMeshComponent|GetStaticMesh (Variables|/Script/Engine.StaticMeshActor|GetStaticMeshComponent _asstatic_mesh_actor)))
        (for (_array_element_2 _array_index) (Variables|Default|GetRandom_Objects) :!label _label
          (if (== _array_element_2 (LocalVariables|GetstaticMesh))
            (CallFunction|MeshSwap (Utilities|Array|Get(acopy) (Variables|Default|GetRandom_Objects) _array_index))
            (bind _ashider (Utilities|Casting|CastToHider (Components|GetOwner)))
            (Default|AdjustWalkSpeed _ashider)
            (Audio|SpawnSoundatLocation "/Game/Sounds/Pop__Morph_.Pop__Morph_" (Transformation|GetActorLocation (Components|GetOwner))))))
      (:CastFailed
        (bind _asreplaceable_mesh_actor (Utilities|Casting|CastToReplaceableMeshActor (.HitActor (Collision|BreakHitResult _outhit)))
          (:then
            (LocalVariables|SetstaticMesh (Variables|/Script/Engine.StaticMeshComponent|GetStaticMesh (Variables|/Game/Blueprints/Daniel/RandomObjectsRoom/ReplaceableMeshActor.ReplaceableMeshActor_C|GetStaticMesh _asreplaceable_mesh_actor)))
            (goto _label))
          (:CastFailed
            (bind _outactors_2 (Actor|GetAllActorsOfClass "/Game/Blueprints/Sudeep/Decoy.Decoy_C"))
            (for _array_element_3 _outactors_2
              (if (== _array_element_3 (.HitActor (Collision|BreakHitResult _outhit)))
                (for _array_element_4 (Actor|GetComponentsByClass _array_element_3 "/Script/Engine.StaticMeshComponent")
                  (CallFunction|MeshSwap (Variables|/Script/Engine.StaticMeshComponent|GetStaticMesh _array_element_4))
                  (bind _ashider_2 (Utilities|Casting|CastToHider (Components|GetOwner)))
                  (Default|AdjustWalkSpeed _ashider_2)
                  (Audio|SpawnSoundatLocation "/Game/Sounds/Pop__Morph_.Pop__Morph_" (Transformation|GetActorLocation (Components|GetOwner))))))))))))

(fn OnRepCurrentObject)

(fn SmokeScreen
  (bind _returnvalue (Components|GetOwner))
  ;[1 1 1] SmokeScreen
  (Game|SpawnActorfromClass "/Game/Blueprints/Sudeep/Smoke_Screen.Smoke_Screen_C" (Math|Transform|MakeTransform (- (Transformation|GetActorLocation _returnvalue) "0,-50.000000,0.000000") (Transformation|GetActorRotation _returnvalue)) "AlwaysSpawn" 0 0))

(fn SpawnDecoy
  (bind _returnvalue (Components|GetOwner))
  (bind _returnvalue_2 (Transformation|GetActorLocation _returnvalue))
  (bind (_x _y) (Math|Vector|BreakVector _returnvalue_2))
  ;[1 1 1] Spawn Decoy
  (for _array_element (Actor|GetComponentsByClass _returnvalue "/Script/Engine.CameraComponent")
    (bind _ashider (Utilities|Casting|CastToHider (Components|GetOwner)))
    (Game|SpawnActorfromClass "/Game/Blueprints/Sudeep/Decoy.Decoy_C" (Math|Transform|MakeTransform (+ (+ _returnvalue_2 "0.000000,0.000000,-90.000000") (* (Math|Vector|Normalize (- (Math|Vector|MakeVector _x _y 0.0) (Math|Vector|MakeVector (.X (Math|Vector|BreakVector (Transformation|GetWorldLocation _array_element))) (.Y (Math|Vector|BreakVector (Transformation|GetWorldLocation _array_element))) 0.0))) 150)) (Transformation|GetActorRotation _returnvalue) "1.000000,1,1.000000") "AlwaysSpawn" 0 _ashider 0)))

(fn Invisible
  ;[1 1 1] Invisible
  (bind _ashider (Utilities|Casting|CastToHider (Components|GetOwner)))
  (CallFunction|MakeInvisible (Variables|/Game/HiderBP/Blueprints/Hider.Hider_C|GetStaticMesh _ashider)))

(fn SilenceTrap
  (bind _returnvalue (Components|GetOwner))
  ;[1 1 1] Silence Trap
  (Game|SpawnActorfromClass "/Game/Blueprints/Sudeep/SilenceTrap.SilenceTrap_C" (Math|Transform|MakeTransform (- (Transformation|GetActorLocation _returnvalue) "0,0.000000,100.000000") (Transformation|GetActorRotation _returnvalue)) "Undefined" 0 0))

(fn FireAmmo
  ;[1 1 1] Fire Ammo
  (switch int (Variables|Default|GetAmmoID)
    (:0
      (CallFunction|SmokeScreen))
    (:1
      (CallFunction|SilenceTrap))))